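; Blueprint function library that handles overlaps between obstacles and ships or bullets.
; Overlap begin and end tell the player ship pawn or enemy ship that it has entered or exited an obstacle.
; A bullet overlap damages the obstacle through HurtMe if it is a Building, then calls BulletDestroy.
; BulletDestroy currently does nothing, as its BP_BasicBullet destroy logic is disconnected.
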(fn ObstacleOverlapBegin
  (params (Actor :type Actor%20Object%20Reference) (Obstacle :type Obstacle%20Object%20Reference))
  (bind _asship_pawn_blueprint (Utilities|Casting|CastToShipPawnBlueprint Actor)
    (:then
      (Default|EnterObstacle _asship_pawn_blueprint))
    (:CastFailed
      (bind _asbp_enemy_ship (Utilities|Casting|CastToBP_EnemyShip Actor)
        (:then
          (Default|EnterObstacle _asbp_enemy_ship))
        (:CastFailed
          (bind _asbullet (Utilities|Casting|CastToBullet Actor))
          (CallFunction|ObstacleDamage Obstacle)
          (CallFunction|BulletDestroy _asbullet))))))

(fn ObstacleOverlapEnd
  (params (Actor :type Actor%20Object%20Reference) (Obstacle :type Obstacle%20Object%20Reference))
  (bind _asship_pawn_blueprint (Utilities|Casting|CastToShipPawnBlueprint Actor)
    (:then
      (Default|ExitObstacle _asship_pawn_blueprint))
    (:CastFailed
      (bind _asbp_enemy_ship (Utilities|Casting|CastToBP_EnemyShip Actor))
      (Default|ExitObstacle _asbp_enemy_ship))))

(fn ObstacleDamage
  (params (Obstacle :type Obstacle%20Object%20Reference))
  (bind _asbuilding (Utilities|Casting|CastToBuilding Obstacle))
  (Default|HurtMe _asbuilding))

(fn BulletDestroy
  (params (Bullet :type Bullet%20Object%20Reference)))