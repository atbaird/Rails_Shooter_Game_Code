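; Game mode for a rails shooter that sets up the player's ship and rails camera when play begins.
; It reuses the first rails camera and ship pawn found in the level, spawning either at a fixed transform near the origin if none exists.
; Player controller 0 then possesses the ship while its view target is set to the separate camera actor.
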(event Custom|Possess%20First%20Ship%20and%20Camera
  (bind _returnvalue (Game|GetPlayerController 0))
  ;[1 1 1] Possess First Ship and Camera
  (if (Utilities|IsValid _returnvalue)
    (Pawn|Possess _returnvalue (Variables|Default|GetShip))
    (Game|Player|SetViewTargetwithBlend _returnvalue (Variables|Default|GetCamera) 0.0 "VTBlend_Linear" 0.0 false)))

(event Custom|GuaranteeRailsCamera
  ;[1 1 1] Guarantee Rails Camera Exists
  (bind _outactors (Actor|GetAllActorsOfClass "/Game/Blueprint/Cameras/RailsCameraBlueprint.RailsCameraBlueprint_C"))
  (if (> (Utilities|Array|Length _outactors) 0)
    (Variables|Default|SetCamera (Utilities|Array|Get(acopy) _outactors))
    (else
      (bind _returnvalue (Game|SpawnActorfromClass "/Game/Blueprint/Cameras/RailsCameraBlueprint.RailsCameraBlueprint_C" (Math|Transform|MakeTransform "0, 0,1.000000" "0,90.000000, 0") "Undefined" 0 0))
      (Variables|Default|SetCamera _returnvalue))))

(event Custom|GuaranteeShipExists
  ;[1 1 1] Guarantee Ship Exists
  (bind _outactors (Actor|GetAllActorsOfClass "/Game/Blueprint/Pawns/ShipPawnBlueprint.ShipPawnBlueprint_C"))
  (if (> (Utilities|Array|Length _outactors) 0)
    (Variables|Default|SetShip (Utilities|Array|Get(acopy) _outactors))
    (else
      (bind _returnvalue (Game|SpawnActorfromClass "/Game/Blueprint/Pawns/ShipPawnBlueprint.ShipPawnBlueprint_C" (Math|Transform|MakeTransform "0, 0,1.000000") "Undefined" 0 0))
      (Variables|Default|SetShip _returnvalue))))

(event EventBeginPlay
  ;[1 1 1] EventbeginPlay
  (CallFunction|GuaranteeRailsCamera)
  (CallFunction|GuaranteeShipExists)
  (CallFunction|PossessFirstShipandCamera))

(fn ConstructionScript)