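; BP_HealthPickup is a powerup that restores health to whoever is picking it up.
; Each Tick it checks for a valid BeingPickedUpBy below MaxHP, adds AmountToHeal capped at MaxHP, then destroys itself.
; At full health the pickup stays in the world, and nothing in these graphs assigns BeingPickedUpBy.
; The construction script applies a blue material to the powerup mesh.
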(event EventBeginPlay)

(event Collision|EventActorBeginOverlap
  (params (OtherActor :type Actor%20Object%20Reference)))

(event EventTick
  (params (DeltaSeconds :type Float%20%28single-precision%29))
  (bind _beingpickedupby (Variables|Default|GetbeingPickedUpBy))
  (bind _beingpickedupby_2 (Variables|Default|GetbeingPickedUpBy))
  (bind _maxhp (Variables|/Script/RailsShooter.PlayerShipNoControlsWithin|GetmaxHP _beingpickedupby))
  (if (Utilities|IsValid _beingpickedupby)
    (if (< (Variables|/Script/RailsShooter.PlayerShipNoControlsWithin|GetcurrentHP _beingpickedupby) _maxhp)
      (if (> (+ (Variables|/Script/RailsShooter.PlayerShipNoControlsWithin|GetcurrentHP _beingpickedupby) (Variables|Default|GetAmountToHeal)) _maxhp)
        (Variables|/Script/RailsShooter.PlayerShipNoControlsWithin|SetcurrentHP _beingpickedupby_2 (Variables|/Script/RailsShooter.PlayerShipNoControlsWithin|GetmaxHP _beingpickedupby_2))
        (else
          (Variables|/Script/RailsShooter.PlayerShipNoControlsWithin|SetcurrentHP _beingpickedupby_2 (+ (Variables|/Script/RailsShooter.PlayerShipNoControlsWithin|GetcurrentHP _beingpickedupby) (Variables|Default|GetAmountToHeal)))))
      (Actor|DestroyActor))))

(fn ConstructionScript
  (Rendering|Material|SetMaterial (Variables|Default|GetPowerupMesh) 0 "/Game/Materials/Mat_Blue.Mat_Blue"))