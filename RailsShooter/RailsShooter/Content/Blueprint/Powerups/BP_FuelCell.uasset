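; BP_FuelCell is a fuel powerup that refills the fuel of the ship picking it up.
; Each Tick, once BeingPickedUpBy is valid and casts to ShipPawnBlueprint, it adds AmountOfFuelToRecover to CurrentFuel, capped at MaxFuel.
; It destroys itself only when fuel is applied, so it remains if the ship's tank is full.
; The construction script gives the powerup mesh a yellow material.
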(event EventBeginPlay)

(event EventTick
  (params (DeltaSeconds :type Float%20%28single-precision%29))
  (bind _beingpickedupby (Variables|Default|GetbeingPickedUpBy))
  (if (Utilities|IsValid _beingpickedupby)
    (bind _asship_pawn_blueprint (Utilities|Casting|CastToShipPawnBlueprint _beingpickedupby))
    (if (< (Variables|/Game/Blueprint/Pawns/ShipPawnBlueprint.ShipPawnBlueprint_C|GetCurrentFuel _asship_pawn_blueprint) (Variables|/Game/Blueprint/Pawns/ShipPawnBlueprint.ShipPawnBlueprint_C|GetMaxFuel _asship_pawn_blueprint))
      (if (> (+ (Variables|/Game/Blueprint/Pawns/ShipPawnBlueprint.ShipPawnBlueprint_C|GetCurrentFuel _asship_pawn_blueprint) (Variables|Default|GetAmountOfFuelToRecover)) (Variables|/Game/Blueprint/Pawns/ShipPawnBlueprint.ShipPawnBlueprint_C|GetMaxFuel _asship_pawn_blueprint))
        (Variables|/Game/Blueprint/Pawns/ShipPawnBlueprint.ShipPawnBlueprint_C|SetCurrentFuel _asship_pawn_blueprint (Variables|/Game/Blueprint/Pawns/ShipPawnBlueprint.ShipPawnBlueprint_C|GetMaxFuel _asship_pawn_blueprint))
        (else
          (Variables|/Game/Blueprint/Pawns/ShipPawnBlueprint.ShipPawnBlueprint_C|SetCurrentFuel _asship_pawn_blueprint (+ (Variables|/Game/Blueprint/Pawns/ShipPawnBlueprint.ShipPawnBlueprint_C|GetCurrentFuel _asship_pawn_blueprint) (Variables|Default|GetAmountOfFuelToRecover)))))
      (Actor|DestroyActor))))

(fn ConstructionScript
  (Rendering|Material|SetMaterial (Variables|Default|GetPowerupMesh) 0 "/Game/Materials/Mat_Yellow.Mat_Yellow"))