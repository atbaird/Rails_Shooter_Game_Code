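; Rails camera actor that continuously scrolls along its camera component's forward vector.
; Each Tick it moves by the current movement speed scaled by delta time, without sweeping.
; A SpeedUp flag multiplies that step and takes priority over a SlowDown flag, which divides it.
; Helper functions expose the orthographic view's aspect ratio, width, derived height and half extents.
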(event EventTick
  (params (DeltaSeconds :type Float%20%28single-precision%29))
  (bind _returnvalue (Transformation|GetActorLocation))
  (bind _camera (Variables|Default|GetCamera))
  (bind _currentmovementspeed (Variables|Default|GetCurrentMovementSpeed))
  (bind _returnvalue_2 (Math|Vector|GetForwardVector _camera))
  (bind _returnvalue_3 (* DeltaSeconds _currentmovementspeed))
  (bind _returnvalue_4 (* _returnvalue_2 _returnvalue_3))
  (if (Variables|Default|GetSpeedUp)
    ;[1 1 1] Speedup
    (Transformation|SetActorLocation (+ _returnvalue (* _returnvalue_4 (Variables|Default|GetSpeedUpMultiplier))) false false)
    (elif (Variables|Default|GetSlowDown)
      ;[1 1 1] SlowDown
      (Transformation|SetActorLocation (+ (/ _returnvalue_4 (Variables|Default|GetSlowDownMultiplier)) _returnvalue) false false)
      (else
        ;[1 1 1] Default
        (Transformation|SetActorLocation (+ _returnvalue _returnvalue_4) false false)))))

(event EventBeginPlay)

(fn ConstructionScript)

(fn GetAspectRatio
  (return (Variables|/Script/Engine.CameraComponent|GetAspectRatio (Variables|Default|GetCamera))))

(fn GetOrthoWidth
  (return (Variables|/Script/Engine.CameraComponent|GetOrthoWidth (Variables|Default|GetCamera))))

(fn GetOrthoHeight
  (return (/ (ViewFrustum|GetOrthoWidth) (ViewFrustum|GetAspectRatio))))

(fn GetHalfOrthoWidth
  (return (/ (ViewFrustum|GetOrthoWidth) 2.0)))

(fn GetHalfOrthoHeight
  (return (/ (ViewFrustum|GetOrthoHeight) 2.0)))