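; Rails camera actor Blueprint that exposes its camera's state through variables, apparently for C++ code as the UpdateC++ function name suggests.
; Every Tick it refreshes aspect ratio, orthographic height (width divided by aspect ratio), direction vectors and world position via small getter functions.
; An OffRailsMoveForward event moves the actor along camera forward at the current movement speed without sweeping; its call in this graph is disconnected.
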(event Custom|OffRailsMoveForward
  (params (DeltaSeconds :type Float%20%28single-precision%29))
  ;[1 1 1] OffRailsMoveForward
  (Transformation|SetActorLocation (+ (Transformation|GetActorLocation) (* (Math|Vector|GetForwardVector (Variables|Default|GetCamera)) (* (Variables|Default|GetCurrentMovementSpeed) DeltaSeconds))) false false))

(event EventBeginPlay)

(event Collision|EventActorBeginOverlap
  (params (OtherActor :type Actor%20Object%20Reference)))

(event EventTick
  (params (DeltaSeconds :type Float%20%28single-precision%29))
  ;[1 1 1] Event Tick
  (CallFunction|UpdateC++))

(fn ConstructionScript)

(fn GetOrthoWidth
  (return (Variables|/Script/Engine.CameraComponent|GetOrthoWidth (Variables|Default|GetCamera))))

(fn GetOrthoHeight
  (return (/ (CameraView|GetOrthoWidth) (CameraView|GetAspectRatio))))

(fn GetAspectRatio
  (return (Variables|/Script/Engine.CameraComponent|GetAspectRatio (Variables|Default|GetCamera))))

(fn GetCameraForward
  (return (Math|Vector|GetForwardVector (Variables|Default|GetCamera))))

(fn GetCameraRight
  (return (Math|Vector|GetRightVector (Variables|Default|GetCamera))))

(fn GetCameraUp
  (return (Math|Vector|GetUpVector (Variables|Default|GetCamera))))

(fn GetCameraWorldPosition
  (return (Transformation|GetWorldLocation (Variables|Default|GetCamera))))

(fn UpdateC++
  (Variables|Default|SetcameraAspectRatio (CameraView|GetAspectRatio))
  (Variables|Default|SetcameraOrthoHeight (CameraView|GetOrthoHeight))
  (Variables|Default|SetcameraAspectRatio (CameraView|GetAspectRatio))
  (Variables|Default|SetCameraForward (CameraView|GetCameraForward))
  (Variables|Default|SetCameraRight (CameraView|GetCameraRight))
  (Variables|Default|SetCameraUp (CameraView|GetCameraUp))
  (Variables|Default|SetCameraWorldPosition (CameraView|GetCameraWorldPosition)))