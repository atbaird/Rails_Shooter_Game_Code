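; Player ship pawn for a rail shooter, flying in a screen-clamped plane ahead of the RailsCameraBlueprint and tilting with input.
; Each tick it positions itself from the camera, spawns two reticle billboards at start, and fires bullets in data-table patterns, reverting to default when scatter ammo runs out.
; Speed-up and slow-down inputs drive the camera's speed, burning fuel that recharges after a delay.
; Being hurt by obstacles shakes the camera.
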(event Custom|ShootingTest
  (params (deltaSeconds :type Float%20%28single-precision%29))
  (bind _secondsbeforecanshoot (Variables|Shoot|GetSecondsBeforeCanShoot))
  ;[1 1 1] ShootingTest
  (if (< (Variables|Shoot|GetSecondsSinceLastShot_0) _secondsbeforecanshoot)
    (Variables|Shoot|SetSecondsSinceLastShot_0 (+ (Variables|Shoot|GetSecondsSinceLastShot_0) deltaSeconds)))
  (if (and (Variables|Shoot|GetwantsToShoot) (>= (Variables|Shoot|GetSecondsSinceLastShot_0) _secondsbeforecanshoot))
    (bind _canshoot (CallFunction|VerifyCanShoot))
    (if _canshoot
      _
      (else
        (Variables|Default|SetCurrentBulletArrangment 0)))
    (CallFunction|SpawnBullet)
    (Variables|Shoot|SetSecondsSinceLastShot_0 0.0)))

(event Custom|SpawnBullet
  (bind _bulletarrangements (Variables|Default|GetBulletArrangements))
  (bind _currentbulletarrangment (Variables|Default|GetCurrentBulletArrangment))
  (bind _item (Utilities|Array|Get(acopy) _bulletarrangements _currentbulletarrangment))
  (bind (_rotationsfromforward _distancesfromrotation) (Utilities|Struct|BreakStruc_BulletArrangement _item))
  (bind _returnvalue (Utilities|Array|Length _rotationsfromforward))
  (bind _returnvalue_2 (Utilities|Array|Length _distancesfromrotation))
  ;[1 1 1] SpawnBullet
  (Variables|Default|SetLoopThrough _returnvalue_2)
  (if (< _returnvalue _returnvalue_2)
    (Variables|Default|SetLoopThrough _returnvalue))
  (for _index (range 0 (Variables|Default|GetLoopThrough))
    (Game|SpawnActorfromClass "/Game/Blueprint/Bullets/BP_BasicBullet.BP_BasicBullet_C" (Math|Transform|MakeTransform (+ (Transformation|GetActorLocation) (* (Math|Vector|GetForwardVector (Math|Rotator|CombineRotators (Transformation|GetActorRotation) (Utilities|Array|Get(acopy) _rotationsfromforward _index))) (Utilities|Array|Get(acopy) _distancesfromrotation _index))) (Math|Rotator|CombineRotators (Transformation|GetActorRotation) (Utilities|Array|Get(acopy) _rotationsfromforward _index))) "Undefined" 0 self)))

(event Custom|FuelTest
  (params (DeltaSeconds :type Float%20%28single-precision%29))
  (bind _worldcamera (Variables|RailsCamera|GetWorldCamera))
  (bind _worldcamera_2 (Variables|RailsCamera|GetWorldCamera))
  (bind _refuelpersecond (Variables|Fuel|GetRefuelPerSecond))
  (bind _worldcamera_3 (Variables|RailsCamera|GetWorldCamera))
  (bind _returnvalue (* _refuelpersecond DeltaSeconds))
  ;[1 1 1] FuelTest
  (if (or (and (Variables|InputSpeedSlow|GetSpeedUp) (not (Variables|InputSpeedSlow|GetSlowDown))) (and (Variables|InputSpeedSlow|GetSlowDown) (not (Variables|InputSpeedSlow|GetSpeedUp))))
    ;;[1 1 1] ExpendFuel
    (Variables|Fuel|SetSecondsSinceStoppedBurningFuel 0.0)
    (if (>= (- (Variables|Fuel|GetCurrentFuel) (* DeltaSeconds (Variables|Fuel|GetFuelPerSecond))) 0.0)
      (Variables|Fuel|SetCurrentFuel (- (Variables|Fuel|GetCurrentFuel) (* DeltaSeconds (Variables|Fuel|GetFuelPerSecond))))
      (if (and (Variables|InputSpeedSlow|GetSpeedUp) (not (Variables|InputSpeedSlow|GetSlowDown)))
        (Variables|/Game/Blueprint/Cameras/RailsCameraBlueprint.RailsCameraBlueprint_C|SetSpeedUp _worldcamera_2 true)
        (Variables|/Game/Blueprint/Cameras/RailsCameraBlueprint.RailsCameraBlueprint_C|SetSlowDown _worldcamera_2 false)
        (elif (and (not (Variables|InputSpeedSlow|GetSpeedUp)) (Variables|InputSpeedSlow|GetSlowDown))
          (Variables|/Game/Blueprint/Cameras/RailsCameraBlueprint.RailsCameraBlueprint_C|SetSlowDown _worldcamera_2 true)
          (Variables|/Game/Blueprint/Cameras/RailsCameraBlueprint.RailsCameraBlueprint_C|SetSpeedUp _worldcamera_2 false)
          (else
            (Variables|/Game/Blueprint/Cameras/RailsCameraBlueprint.RailsCameraBlueprint_C|SetSlowDown _worldcamera_2 false)
            (Variables|/Game/Blueprint/Cameras/RailsCameraBlueprint.RailsCameraBlueprint_C|SetSpeedUp _worldcamera_2 false))))
      (else
        (Variables|Fuel|SetCurrentFuel 0.0)
        (Variables|/Game/Blueprint/Cameras/RailsCameraBlueprint.RailsCameraBlueprint_C|SetSlowDown _worldcamera false)
        (Variables|/Game/Blueprint/Cameras/RailsCameraBlueprint.RailsCameraBlueprint_C|SetSpeedUp _worldcamera false)))
    (else
      (Variables|/Game/Blueprint/Cameras/RailsCameraBlueprint.RailsCameraBlueprint_C|SetSpeedUp _worldcamera_3 false)
      (Variables|/Game/Blueprint/Cameras/RailsCameraBlueprint.RailsCameraBlueprint_C|SetSlowDown _worldcamera_3 false)
      (Variables|Fuel|SetSecondsSinceStoppedBurningFuel (+ DeltaSeconds (Variables|Fuel|GetSecondsSinceStoppedBurningFuel)))
      ;;[1 1 1] Refuel
      (if (and (< (Variables|Fuel|GetCurrentFuel) (Variables|Fuel|GetMaxFuel)) (>= (Variables|Fuel|GetSecondsSinceStoppedBurningFuel) (Variables|Fuel|GetSecondsBeforeStartChargingFuel)))
        (if (> _returnvalue (Variables|Fuel|GetMaxFuel))
          (Variables|Fuel|SetCurrentFuel (Variables|Fuel|GetMaxFuel))
          (else
            (Variables|Fuel|SetCurrentFuel (+ (Variables|Fuel|GetCurrentFuel) _returnvalue))))))))

(event Custom|SetScatterShotAmmoToMax
  (bind _bulletarrangements (Variables|Default|GetBulletArrangements))
  (bind _item (Utilities|Array|Get(acopy) _bulletarrangements 1))
  (bind (_rotationsfromforward _distancesfromrotation _startingammo _maxammo) (Utilities|Struct|BreakStruc_BulletArrangement _item))
  ;[1 1 1] SetScatterShotAmmoToMax
  (Utilities|Array|SetArrayElem (Variables|Default|GetBulletArrangements) 1 (Utilities|Struct|MakeStruc_BulletArrangement _rotationsfromforward _distancesfromrotation _startingammo _maxammo _maxammo))
  (Variables|Default|SetCurrentBulletArrangment 1))

(event Custom|EnterObstacle
  (Class|PlayerShipNoControlsWithin|EnteredObstacle))

(event Custom|ExitObstacle
  (Class|PlayerShipNoControlsWithin|ExitedObstacle))

(event Custom|Spawn%20and%20Set%20up%20reticle
  (bind _self self)
  ;[1 1 1] Spawn and Set Up Reticle
  ;;[1 1 1] Spawn Reticle Billboards
  (if (!= self 0)
    (bind _returnvalue (Game|SpawnActorfromClass "/Game/Blueprint/BP_ReticleBillboard.BP_ReticleBillboard_C" (Math|Transform|MakeTransform "0, 0, 0") "Undefined" 0 0))
    (Variables|Reticle|SetbigReticle _returnvalue)
    (bind _returnvalue_2 (Game|SpawnActorfromClass "/Game/Blueprint/BP_ReticleBillboard.BP_ReticleBillboard_C" (Math|Transform|MakeTransform "0, 0, 0" "0, 0, 0" "1.000000,1.000000,1.000000") "Undefined" 0 0))
    (Variables|Reticle|SetsmallReticle _returnvalue_2)
    ;;[1 1 1] Set To Go Out From
    (Variables|/Script/RailsShooter.ReticleBillboards|SetToGoOutFrom (Variables|Reticle|GetbigReticle) _self)
    (Variables|/Script/RailsShooter.ReticleBillboards|SetToGoOutFrom (Variables|Reticle|GetsmallReticle) _self)
    ;;[1 1 1] Distance to Maintain
    (Variables|/Script/RailsShooter.ReticleBillboards|SetdistanceToMaintain (Variables|Reticle|GetbigReticle) 2.5e+02)
    (Variables|/Script/RailsShooter.ReticleBillboards|SetdistanceToMaintain (Variables|Reticle|GetsmallReticle) 5e+02)
    ;;[1 1 1] Scale
    (Transformation|SetActorRelativeScale3D (Variables|Reticle|GetbigReticle) "1.000000,1.000000,1.000000")
    (Transformation|SetActorRelativeScale3D (Variables|Reticle|GetsmallReticle) "0.500000,0.500000,0.500000")))

(event EventBeginPlay
  (bind _bulletarrangements (Variables|Default|GetBulletArrangements))
  ;[1 1 1] Event beginplay
  ;;[1 1 1] Get Camera
  (bind _outactors (Actor|GetAllActorsOfClass "/Game/Blueprint/Cameras/RailsCameraBlueprint.RailsCameraBlueprint_C"))
  (if (> (Utilities|Array|Length _outactors) 0)
    (bind _output_get (Variables|RailsCamera|SetWorldCamera (Utilities|Array|Get(acopy) _outactors)))
    (Variables|/Game/Blueprint/Cameras/RailsCameraBlueprint.RailsCameraBlueprint_C|SetSpeedUp _output_get false)
    ;;[1 1 1] Place Ship in front of Camera
    (RelationToCamera|SetRelativePositionCentertoCamera)
    ;;[1 1 1] Set Default Position
    (RelationToCamera|SetShiptoDefaultDistanceinFrontOfCamera)
    (Variables|Shoot|SetSecondsSinceLastShot_0 (Variables|Shoot|GetSecondsBeforeCanShoot))
    ;;[1 1 1] Spawn and Set Up Reticle
    (CallFunction|SpawnandSetUpReticle)
    (Variables|Fuel|SetCurrentFuel (Variables|Fuel|GetMaxFuel))
    (bind _returnvalue (Utilities|GetDataTableRow "/Game/Blueprint/Bullets/DataTable_BulletArrangemnets.DataTable_BulletArrangemnets" "Default")
      (:then
        (Utilities|Array|AddUnique _bulletarrangements _returnvalue)
        (bind _returnvalue_2 (Utilities|GetDataTableRow "/Game/Blueprint/Bullets/DataTable_BulletArrangemnets.DataTable_BulletArrangemnets" "Scatter")
          (:then
            (Utilities|Array|AddUnique _bulletarrangements _returnvalue_2)))))))

(event EventDestroyed
  ;[1 1 1] Event Destroyed
  (Actor|DestroyActor (Variables|Reticle|GetbigReticle))
  (Actor|DestroyActor (Variables|Reticle|GetsmallReticle)))

(event EventTick
  (params (DeltaSeconds :type Float%20%28single-precision%29))
  ;[1 1 1] Event Tick
  (if (Variables|Default|GetjustHurtByObstacle)
    (Camera|PlayWorldCameraShake "/Game/Blueprint/Cameras/BP_CamShake.BP_CamShake_C" (Transformation|GetActorLocation (Variables|RailsCamera|GetWorldCamera)) 0.0 5e+02 1.0))
  (CallFunction|FuelTest DeltaSeconds)
  (bind _asbp_controller (Utilities|Casting|CastToBP_Controller (Pawn|GetController)))
  (Variables|Default|SetmyController _asbp_controller)
  (CallFunction|UpdateMovement DeltaSeconds)
  (bind (_shipposition _shiprotation) (RelationToCamera|GetShipPositionandRotationfromCamera))
  (Transformation|SetActorLocationAndRotation _shipposition _shiprotation)
  (CallFunction|ShootingTest DeltaSeconds))

(event Input|ActionEvents|InputActionShoot
  (params (Key :type Key%20Structure :default "AnyKey"))
  ;[1 1 1] Shoot
  (:Pressed
    (Variables|Shoot|SetSecondsSinceLastShot_0 (Variables|Shoot|GetSecondsBeforeCanShoot))
    (Variables|Shoot|SetwantsToShoot true))
  (:Released
    (Variables|Shoot|SetwantsToShoot false)))

(event Input|ActionEvents|InputActionSpeedUp
  (params (Key :type Key%20Structure :default "AnyKey"))
  ;[1 1 1] SpeedUp
  (:Pressed
    (Variables|InputSpeedSlow|SetSpeedUp true))
  (:Released
    (Variables|InputSpeedSlow|SetSpeedUp false)))

(event Input|ActionEvents|InputActionSlowDown
  (params (Key :type Key%20Structure :default "AnyKey"))
  ;[1 1 1] SlowDown
  (:Pressed
    (Variables|InputSpeedSlow|SetSlowDown true))
  (:Released
    (Variables|InputSpeedSlow|SetSlowDown false)))

(event Input|AxisEvents|InputAxisMoveUp
  (params (AxisValue :type Float%20%28single-precision%29))
  ;[1 1 1] MoveUp
  (Variables|MovementRelated|SetCurrentMovementInput (Math|Vector2D|MakeVector2D (.X (Math|Vector2D|BreakVector2D (Variables|MovementRelated|GetCurrentMovementInput))) (Math|Float|Clamp(Float) AxisValue -1.0))))

(event Input|AxisEvents|InputAxisMoveRight
  (params (AxisValue :type Float%20%28single-precision%29))
  ;[1 1 1] MoveRight
  (Variables|MovementRelated|SetCurrentMovementInput (Math|Vector2D|MakeVector2D (Math|Float|Clamp(Float) AxisValue -1.0) (.Y (Math|Vector2D|BreakVector2D (Variables|MovementRelated|GetCurrentMovementInput))))))

(fn ConstructionScript
  ;[1 1 1] Comment
  (bind _outactors (Actor|GetAllActorsOfClass "/Game/Blueprint/Cameras/RailsCameraBlueprint.RailsCameraBlueprint_C"))
  (if (> (Utilities|Array|Length _outactors) 0)
    (Variables|RailsCamera|SetWorldCamera (Utilities|Array|Get(acopy) _outactors)))
  ;[1 1 1] Place Ship in front of Camera
  (RelationToCamera|SetRelativePositionCentertoCamera)
  ;[1 1 1] Set Default Position
  (RelationToCamera|SetShiptoDefaultDistanceinFrontOfCamera)
  (Variables|Shoot|SetSecondsSinceLastShot_0 (Variables|Shoot|GetSecondsBeforeCanShoot)))

(fn SetShiptoDefaultDistanceinFrontOfCamera
  (bind (_shipposition _shiprotation) (RelationToCamera|GetShipPositionandRotationfromCamera))
  (Transformation|SetActorLocationAndRotation _shipposition _shiprotation))

(fn SetRelativePositionCentertoCamera
  (bind _worldcamera (Variables|RailsCamera|GetWorldCamera))
  (if (Utilities|IsValid _worldcamera)
    (Variables|PositionFromCamera|SetRelativeScreenPosition (Math|Vector2D|MakeVector2D (Default|GetHalfOrthoWidth _worldcamera) (Default|GetHalfOrthoHeight _worldcamera)))))

(fn GetShipPositionandRotationfromCamera
  (bind _relativescreenposition (Variables|PositionFromCamera|GetRelativeScreenPosition))
  (bind _worldcamera (Variables|RailsCamera|GetWorldCamera))
  (bind _worldcamera_2 (Variables|RailsCamera|GetWorldCamera))
  (bind _currentmovementinput (Variables|MovementRelated|GetCurrentMovementInput))
  (bind _amountcantilt (Variables|Default|GetamountCanTilt))
  (bind _worldcamera_3 (Variables|RailsCamera|GetWorldCamera))
  (bind (_x _y) (Math|Vector2D|BreakVector2D _relativescreenposition))
  (bind _returnvalue (* _currentmovementinput _amountcantilt))
  (bind _camera (Variables|/Game/Blueprint/Cameras/RailsCameraBlueprint.RailsCameraBlueprint_C|GetCamera _worldcamera_3))
  (bind _camera_2 (Variables|/Game/Blueprint/Cameras/RailsCameraBlueprint.RailsCameraBlueprint_C|GetCamera _worldcamera))
  (bind _camera_3 (Variables|/Game/Blueprint/Cameras/RailsCameraBlueprint.RailsCameraBlueprint_C|GetCamera _worldcamera_2))
  (bind _returnvalue_2 (Math|Vector|GetForwardVector _camera_3))
  (bind _returnvalue_3 (Math|Vector|GetUpVector _camera_3))
  (bind _returnvalue_4 (Math|Vector|GetRightVector _camera_3))
  (bind (_x_2 _y_2) (Math|Vector2D|BreakVector2D _returnvalue))
  (bind _returnvalue_5 (Math|Rotator|MakeRotationfromAxes _returnvalue_2 _returnvalue_4 _returnvalue_3))
  (bind (_roll _pitch _yaw) (Math|Rotator|BreakRotator _returnvalue_5))
  ;[1 1 1] Verify Camera not null
  (if (Utilities|IsValid _worldcamera_3)
    (return (+ (Transformation|GetWorldLocation _camera) (* (Math|Vector|GetForwardVector _camera) (Variables|PositionFromCamera|GetDistanceForwardFromCamera)) (* (Math|Vector|GetRightVector _camera_2) (- _x (Default|GetHalfOrthoWidth _worldcamera))) (* (Math|Vector|GetUpVector _camera_2) (- _y (Default|GetHalfOrthoHeight _worldcamera)))) (Math|Rotator|MakeRotator _roll (+ _pitch _y_2) (+ _yaw _x_2)))
    (else
      (return (Transformation|GetActorLocation) (Transformation|GetActorRotation)))))

(fn UpdateMovement
  (params (deltaSeconds :type Float%20%28single-precision%29))
  (bind _currentmovementinput (Variables|MovementRelated|GetCurrentMovementInput))
  (bind _movementspeedmultiplier (Variables|MovementRelated|GetMovementSpeedMultiplier))
  (bind _worldcamera (Variables|RailsCamera|GetWorldCamera))
  (bind _worldcamera_2 (Variables|RailsCamera|GetWorldCamera))
  (bind _returnvalue (Math|Vector2D|Normalize2D _currentmovementinput))
  (bind _orthowidth (Default|GetOrthoWidth _worldcamera))
  (bind _orthoheight (Default|GetOrthoHeight _worldcamera_2))
  (bind _returnvalue_2 (* _movementspeedmultiplier deltaSeconds))
  (bind _returnvalue_3 (* _returnvalue _returnvalue_2))
  (bind (_x _y) (Math|Vector2D|BreakVector2D _returnvalue_3))
  (if (Utilities|IsValid (Variables|RailsCamera|GetWorldCamera))
    (Utilities|FlowControl|Sequence
      (:then_0
        ;[1 1 1] X Movement Update
        (if (< (+ _x (.X (Math|Vector2D|BreakVector2D (Variables|PositionFromCamera|GetRelativeScreenPosition)))) 0.0)
          ;;[1 1 1] Less than min width
          (Variables|PositionFromCamera|SetRelativeScreenPosition (Math|Vector2D|MakeVector2D 0.0 (.Y (Math|Vector2D|BreakVector2D (Variables|PositionFromCamera|GetRelativeScreenPosition)))))
          (elif (> (+ _x (.X (Math|Vector2D|BreakVector2D (Variables|PositionFromCamera|GetRelativeScreenPosition)))) _orthowidth)
            ;;[1 1 1] Greater than ortho width
            (Variables|PositionFromCamera|SetRelativeScreenPosition (Math|Vector2D|MakeVector2D _orthowidth (.Y (Math|Vector2D|BreakVector2D (Variables|PositionFromCamera|GetRelativeScreenPosition)))))
            (else
              (Variables|PositionFromCamera|SetRelativeScreenPosition (Math|Vector2D|MakeVector2D (+ _x (.X (Math|Vector2D|BreakVector2D (Variables|PositionFromCamera|GetRelativeScreenPosition)))) (.Y (Math|Vector2D|BreakVector2D (Variables|PositionFromCamera|GetRelativeScreenPosition)))))))))
      (:then_1
        ;[1 1 1] Y Movement Update
        (if (< (+ _y (.Y (Math|Vector2D|BreakVector2D (Variables|PositionFromCamera|GetRelativeScreenPosition)))) 0.0)
          ;;[1 1 1] Less than Min Height
          (Variables|PositionFromCamera|SetRelativeScreenPosition (Math|Vector2D|MakeVector2D (.X (Math|Vector2D|BreakVector2D (Variables|PositionFromCamera|GetRelativeScreenPosition))) 0.0))
          (elif (> (+ _y (.Y (Math|Vector2D|BreakVector2D (Variables|PositionFromCamera|GetRelativeScreenPosition)))) _orthoheight)
            ;;[1 1 1] Greater than Max Height
            (Variables|PositionFromCamera|SetRelativeScreenPosition (Math|Vector2D|MakeVector2D (.X (Math|Vector2D|BreakVector2D (Variables|PositionFromCamera|GetRelativeScreenPosition))) _orthoheight))
            (else
              (Variables|PositionFromCamera|SetRelativeScreenPosition (Math|Vector2D|MakeVector2D (.X (Math|Vector2D|BreakVector2D (Variables|PositionFromCamera|GetRelativeScreenPosition))) (+ _y (.Y (Math|Vector2D|BreakVector2D (Variables|PositionFromCamera|GetRelativeScreenPosition)))))))))))))

(fn VerifyCanShoot
  (bind _currentbulletarrangment (Variables|Default|GetCurrentBulletArrangment))
  (bind _bulletarrangements (Variables|Default|GetBulletArrangements))
  (bind _item (Utilities|Array|Get(acopy) _bulletarrangements _currentbulletarrangment))
  (bind (_rotationsfromforward _distancesfromrotation _startingammo _maxammo _currentammo) (Utilities|Struct|BreakStruc_BulletArrangement _item))
  (LocalVariables|SetCurrentAmmo _currentammo)
  (if (>= (LocalVariables|GetCurrentAmmo) 0)
    (if (> (LocalVariables|GetCurrentAmmo) 0)
      (Utilities|Array|SetArrayElem (Variables|Default|GetBulletArrangements) (Variables|Default|GetCurrentBulletArrangment) (Utilities|Struct|MakeStruc_BulletArrangement _rotationsfromforward _distancesfromrotation _startingammo _maxammo (- (LocalVariables|GetCurrentAmmo) 1)))
      (else
        (return false))))
  (return true))