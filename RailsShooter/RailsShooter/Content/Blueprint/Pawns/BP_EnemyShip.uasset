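; Enemy ship pawn that fires patterned volleys of BP_BasicBullet.
; BeginPlay adds the "Default" row of the bullet arrangement data table to its list of arrangements.
; Fire spawns bullets at the current arrangement's paired rotation and distance offsets, relative to the ship, spending one ammo per volley.
; Negative ammo means infinite, zero reverts to the first arrangement without firing, and obstacle events forward to EnteredObstacle and ExitedObstacle.
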(event Custom|EnterObstacle
  (Class|EnemyShip|EnteredObstacle))

(event Custom|ExitObstacle
  (Class|EnemyShip|ExitedObstacle))

(event EventBeginPlay
  (bind _returnvalue (Utilities|GetDataTableRow "/Game/Blueprint/Bullets/DataTable_BulletArrangemnets.DataTable_BulletArrangemnets" "Default")
    (:then
      (Utilities|Array|AddUnique (Variables|Default|GetBulletArrangments) _returnvalue))))

(event Collision|EventActorBeginOverlap
  (params (OtherActor :type Actor%20Object%20Reference)))

(event EventFire
  ;[1 1 1] Guarantee can shoot
  ;;[1 1 1] infinite ammo test
  (if (>= (.CurrentAmmo (Utilities|Struct|BreakStruc_BulletArrangement (Utilities|Array|Get(acopy) (Variables|Default|GetBulletArrangments) (Variables|Default|GetCurrentBulletArrangement)))) 0)
    (if (> (.CurrentAmmo (Utilities|Struct|BreakStruc_BulletArrangement (Utilities|Array|Get(acopy) (Variables|Default|GetBulletArrangments) (Variables|Default|GetCurrentBulletArrangement)))) 0)
      (Utilities|Array|SetArrayElem (Variables|Default|GetBulletArrangments) (Variables|Default|GetCurrentBulletArrangement) (Utilities|Struct|MakeStruc_BulletArrangement (.RotationsFromForward (Utilities|Struct|BreakStruc_BulletArrangement (Utilities|Array|Get(acopy) (Variables|Default|GetBulletArrangments) (Variables|Default|GetCurrentBulletArrangement)))) (.DistancesFromRotation (Utilities|Struct|BreakStruc_BulletArrangement (Utilities|Array|Get(acopy) (Variables|Default|GetBulletArrangments) (Variables|Default|GetCurrentBulletArrangement)))) (.StartingAmmo (Utilities|Struct|BreakStruc_BulletArrangement (Utilities|Array|Get(acopy) (Variables|Default|GetBulletArrangments) (Variables|Default|GetCurrentBulletArrangement)))) (.MaxAmmo (Utilities|Struct|BreakStruc_BulletArrangement (Utilities|Array|Get(acopy) (Variables|Default|GetBulletArrangments) (Variables|Default|GetCurrentBulletArrangement)))) (- (.CurrentAmmo (Utilities|Struct|BreakStruc_BulletArrangement (Utilities|Array|Get(acopy) (Variables|Default|GetBulletArrangments) (Variables|Default|GetCurrentBulletArrangement)))) 1)))
      (Variables|Default|SetLoopThrough (Utilities|Array|Length (.RotationsFromForward (Utilities|Struct|BreakStruc_BulletArrangement (Utilities|Array|Get(acopy) (Variables|Default|GetBulletArrangments) (Variables|Default|GetCurrentBulletArrangement))))) :!label _label)
      (if (< (Utilities|Array|Length (.DistancesFromRotation (Utilities|Struct|BreakStruc_BulletArrangement (Utilities|Array|Get(acopy) (Variables|Default|GetBulletArrangments) (Variables|Default|GetCurrentBulletArrangement))))) (Utilities|Array|Length (.RotationsFromForward (Utilities|Struct|BreakStruc_BulletArrangement (Utilities|Array|Get(acopy) (Variables|Default|GetBulletArrangments) (Variables|Default|GetCurrentBulletArrangement))))))
        (Variables|Default|SetLoopThrough (Utilities|Array|Length (.DistancesFromRotation (Utilities|Struct|BreakStruc_BulletArrangement (Utilities|Array|Get(acopy) (Variables|Default|GetBulletArrangments) (Variables|Default|GetCurrentBulletArrangement)))))))
      ;[1 1 1] Comment
      (for _index (range 0 (Variables|Default|GetLoopThrough))
        (Game|SpawnActorfromClass "/Game/Blueprint/Bullets/BP_BasicBullet.BP_BasicBullet_C" (Math|Transform|MakeTransform (+ (Transformation|GetActorLocation) (* (Math|Vector|GetForwardVector (Math|Rotator|CombineRotators (Transformation|GetActorRotation) (Utilities|Array|Get(acopy) (.RotationsFromForward (Utilities|Struct|BreakStruc_BulletArrangement (Utilities|Array|Get(acopy) (Variables|Default|GetBulletArrangments) (Variables|Default|GetCurrentBulletArrangement)))) _index))) (Utilities|Array|Get(acopy) (.DistancesFromRotation (Utilities|Struct|BreakStruc_BulletArrangement (Utilities|Array|Get(acopy) (Variables|Default|GetBulletArrangments) (Variables|Default|GetCurrentBulletArrangement)))) _index))) (Math|Rotator|CombineRotators (Transformation|GetActorRotation) (Utilities|Array|Get(acopy) (.RotationsFromForward (Utilities|Struct|BreakStruc_BulletArrangement (Utilities|Array|Get(acopy) (Variables|Default|GetBulletArrangments) (Variables|Default|GetCurrentBulletArrangement)))) _index))) "Undefined" 0 self))
      (else
        (Variables|Default|SetCurrentBulletArrangement 0)))
    (else
      (goto _label))))

(fn ConstructionScript)